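; Player controller that owns the game's UI screens: start, HUD, game over, get item, level up, pause and pre-upgrade menus.
; BeginPlay spawns widgets from a data-driven row list, routes each to its variable through a widget ID message, and adds it with per-row Z-order and visibility.
; Show functions hide all widgets, reveal the relevant ones, layering item and level-up over the HUD, and adjust cursor and input mode.
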(event `self.ReceiveBeginPlay`
  (set `self.bShowMouseCursor` true)
  (for _array_element (`self.WidgetInitRows`)
    (bind _returnvalue (`|CreateWidget` (break `/Game/Blueprints/UI/ST_WidgetInitRow` _array_element)))
    (bind _widgetid (message `/Game/Blueprints/UI/BPI_IdentifiableWidget.GetWidgetID` _returnvalue))
    (switch `/Game/Blueprints/UI/EwidgetID` _widgetid
      (:`NewEnumerator0`
        (set `self.StartMenu` _returnvalue))
      (:`NewEnumerator1`
        (set `self.HUD` _returnvalue))
      (:`NewEnumerator2`
        (set `self.GameOverMenu` _returnvalue))
      (:`NewEnumerator3`
        (set `self.GetItem` _returnvalue))
      (:`NewEnumerator4`
        (set `self.LevelUp` _returnvalue))
      (:`NewEnumerator5`
        (set `self.PauseMenu` _returnvalue))
      (:`NewEnumerator6`
        (set `self.PreUpgradeMenu` _returnvalue)))
    (`UserWidget.AddToViewport` _returnvalue (`.ZOrder_9_974CB75142B86629C7ACBFBC6C2343C6` (break `/Game/Blueprints/UI/ST_WidgetInitRow` _array_element)))
    (`Widget.SetVisibility` _returnvalue (select `bool` (`.bStartVisible_13_2C8905F44A68BD70106FB8B744889A39` (break `/Game/Blueprints/UI/ST_WidgetInitRow` _array_element)) :`false` "Hidden" :`true` "Visible" :!type "ESlateVisibility Enum"))))

(fn `HiddenAllWidget`
  (`Widget.SetVisibility` (`self.GameOverMenu`) "Hidden")
  (`Widget.SetVisibility` (`self.GetItem`) "Hidden")
  (`Widget.SetVisibility` (`self.HUD`) "Hidden")
  (`Widget.SetVisibility` (`self.LevelUp`) "Hidden")
  (`Widget.SetVisibility` (`self.PauseMenu`) "Hidden")
  (`Widget.SetVisibility` (`self.PreUpgradeMenu`) "Hidden")
  (`Widget.SetVisibility` (`self.StartMenu`) "Hidden"))

(fn `ShowGameOverMenuWidget`
  (`self.HiddenAllWidget`)
  (`Widget.SetVisibility` (`self.GameOverMenu`) "Visible")
  (set `self.bShowMouseCursor` true))

(fn `ShowGetItemWidget`
  (`self.HiddenAllWidget`)
  (`Widget.SetVisibility` (`self.HUD`) "Visible")
  (`Widget.SetVisibility` (`self.GetItem`) "Visible")
  (set `self.bShowMouseCursor` true))

(fn `ShowHUDWidget`
  (`self.HiddenAllWidget`)
  (`Widget.SetVisibility` (`self.HUD`) "Visible")
  (set `self.bShowMouseCursor` false)
  (`WidgetBlueprintLibrary.SetInputMode_GameOnly` self))

(fn `ShowLevelUpWidget`
  (`self.HiddenAllWidget`)
  (`Widget.SetVisibility` (`self.HUD`) "Visible")
  (`Widget.SetVisibility` (`self.LevelUp`) "Visible")
  (set `self.bShowMouseCursor` true))

(fn `ShowPauseMenuWidget`
  (`self.HiddenAllWidget`)
  (`Widget.SetVisibility` (`self.PauseMenu`) "Visible")
  (set `self.bShowMouseCursor` true))

(fn `ShowPreUpgradeMenuWidget`
  (`self.HiddenAllWidget`)
  (`Widget.SetVisibility` (`self.PreUpgradeMenu`) "Visible"))

(fn `ShowStartMenuWidget`
  (`self.HiddenAllWidget`)
  (`Widget.SetVisibility` (`self.StartMenu`) "Visible")
  (set `self.bShowMouseCursor` true))

(fn `UserConstructionScript`)